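; Map-load actor for the CopperSlides mod that reskins Slide and AimBeltSlide buildings with a copper metal tube material.
; On BeginPlay it binds to the mod API's loading-finished and building-spawned events.
; When loading finishes it swaps the material on every existing slide of both types.
; Each newly spawned building is cast to both types and gets the same swap if it matches.
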(event Custom|OnLoadingFinished
  (Utilities|FlowControl|Sequence
    (:then_0
      (bind _outactors (Actor|GetAllActorsOfClass "/Game/GridActors/Slide.Slide_C"))
      (for _array_element _outactors
        (Rendering|Material|SetMaterial (Variables|/Game/GridActors/Slide.Slide_C|GetStaticMesh12 _array_element) 0 "/Game/Mods/CopperSlides/MI_Copper_MetalTube.MI_Copper_MetalTube")))
    (:then_1
      (bind _outactors_2 (Actor|GetAllActorsOfClass "/Game/GridActors/aim/AimBeltSlide.AimBeltSlide_C"))
      (for _array_element_2 _outactors_2
        (Rendering|Material|SetMaterial (Variables|/Game/GridActors/aim/AimBeltSlide.AimBeltSlide_C|GetStaticMesh2 _array_element_2) 0 "/Game/Mods/CopperSlides/MI_Copper_MetalTube.MI_Copper_MetalTube")))))

(event Custom|OnSlideSpawned
  (params (Actor :type Actor%20Object%20Reference))
  (Utilities|FlowControl|Sequence
    (:then_0
      (bind _asslide (Utilities|Casting|CastToSlide Actor))
      (Rendering|Material|SetMaterial (Variables|/Game/GridActors/Slide.Slide_C|GetStaticMesh12 _asslide) 0 "/Game/Mods/CopperSlides/MI_Copper_MetalTube.MI_Copper_MetalTube"))
    (:then_1
      (bind _asaim_belt_slide (Utilities|Casting|CastToAimBeltSlide Actor))
      (Rendering|Material|SetMaterial (Variables|/Game/GridActors/aim/AimBeltSlide.AimBeltSlide_C|GetStaticMesh2 _asaim_belt_slide) 0 "/Game/Mods/CopperSlides/MI_Copper_MetalTube.MI_Copper_MetalTube"))))

(event EventBeginPlay
  (EventDispatchers|BindEventtoOnLoadingFinished (Class|ModAPI|GetModAPI) (delegate Custom|OnLoadingFinished))
  (EventDispatchers|BindEventtoOnBuildingSpawned (Class|ModAPI|GetModAPI) (delegate Custom|OnSlideSpawned)))

(fn ConstructionScript)