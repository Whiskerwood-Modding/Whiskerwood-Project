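; Main menu mod Blueprint that demonstrates a localized text widget.
; On BeginPlay it registers an English string with the mod API, then after a short delay adds WBP_WidgetLocalization to the viewport.
; The widget's text comes from the localization manager by key, falling back to the English value when the lookup is empty.
; An option-changed binding removes and rebuilds the widget whenever the language setting changes.
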(event Custom|OnOptionChanged
  (params (optionId :type String) (Value :type String))
  (if (Utilities|Enum|Equal(Enum) optionId "settings.language")
    (Widget|RemovefromParent (Variables|Default|GetWidget))
    (CallFunction|ConstructLocalizedWidget)))

(event EventBeginPlay
  (EventDispatchers|BindEventtoOnOptionChanged (Class|ModAPI|GetModAPI) (delegate Custom|OnOptionChanged))
  (Class|ModAPI|AddNewStrings (Class|ModAPI|GetModAPI) "en" (Utilities|Map|MakeMap (Variables|Default|GetLoc%20Key) (Variables|Default|GetEnglish%20Value)))
  (Utilities|FlowControl|Delay 0.2)
  (CallFunction|ConstructLocalizedWidget))

(fn ConstructionScript)

(fn ConstructLocalizedWidget
  (bind _returnvalue (Class|Backbone|GetLocManager))
  (bind _loc_key (Variables|Default|GetLoc%20Key))
  (bind _returnvalue_2 (Class|LocManager|GetWordfromKey _returnvalue _loc_key))
  (bind _returnvalue_3 (UserInterface|CreateWidget "/Game/Mods/WidgetLocalization/WBP_WidgetLocalization.WBP_WidgetLocalization_C"))
  (bind _output_get (Variables|Default|SetWidget _returnvalue_3))
  (if (Utilities|Array|IsEmpty _returnvalue_2)
    (Rendering|Components|TextRender|SetText (Variables|/Game/Mods/WidgetLocalization/WBP_WidgetLocalization.WBP_WidgetLocalization_C|GettxtOutput (Variables|Default|GetWidget)) (Utilities|Text|ToText(String) (Variables|Default|GetEnglish%20Value)))
    (else
      (Rendering|Components|TextRender|SetText (Variables|/Game/Mods/WidgetLocalization/WBP_WidgetLocalization.WBP_WidgetLocalization_C|GettxtOutput (Variables|Default|GetWidget)) (Utilities|Text|ToText(String) _returnvalue_2))))
  (UserInterface|Viewport|AddtoViewport _output_get 0))