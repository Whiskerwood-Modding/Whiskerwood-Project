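; BP_MapLoad is a PrettierPath mod Blueprint meant to reskin stone paths (FastFloor actors) with a cobblestone material.
; SetMesh casts to FastFloor and replaces the first material slot on its bridge mesh, leaving the mesh itself unchanged.
; Handlers apply it to all existing paths after loading and to spawned buildings.
; The mod API bindings for both handlers sit in unconnected nodes, and BeginPlay is empty.
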(event Custom|OnLoadingFinished
  (bind _outactors (Actor|GetAllActorsOfClass "/Game/GridActors/slimActors/FastFloor.FastFloor_C"))
  (for _array_element _outactors
    (CallFunction|SetMesh _array_element)))

(event Custom|OnStonePathSpawned
  (params (Actor :type Actor%20Object%20Reference))
  (CallFunction|SetMesh Actor))

(event EventBeginPlay)

(fn ConstructionScript)

(fn SetMesh
  (params (Object :type Object%20Object%20Reference))
  (bind _asfast_floor (Utilities|Casting|CastToFastFloor Object))
  (Rendering|Material|SetMaterial (Variables|/Game/GridActors/slimActors/FastFloor.FastFloor_C|GetSM_Bridge_Wooden_01_A3 _asfast_floor) 0 "/Game/Mods/PrettierPath/MI_Cobblestone.MI_Cobblestone"))