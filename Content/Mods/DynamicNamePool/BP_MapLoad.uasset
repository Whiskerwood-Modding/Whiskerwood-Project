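; BP_MapLoad is the DynamicNamePool mod's Blueprint that replaces the game's Whisker name pool with names from a text file.
; On every Tick it re-reads names.txt through the mod API, splits it on commas without empty entries, and passes the array to SetWhiskerNamePool.
; A Log Message helper writes timestamped, mod-tagged lines through the API, but the Tick logic does not call it.
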(event EventTick
  (params (DeltaSeconds :type Float%20%28single-precision%29))
  (bind _returnvalue (Class|ModAPI|ReadModTextFile (Class|ModAPI|GetModAPI) "DynamicNamePool" "names.txt"))
  (Class|ModAPI|SetWhiskerNamePool (Class|ModAPI|GetModAPI) (Utilities|String|ParseIntoArray _returnvalue ",")))

(fn ConstructionScript)

(fn LogMessage
  (params (Message :type String) (Mod%20Name :type String))
  (bind _returnvalue (Math|DateTime|Now))
  (bind (_year _month _day _hour _minute _second _millisecond) (Math|DateTime|BreakDateTime _returnvalue))
  (Class|ModAPI|LogMessage (Class|ModAPI|GetModAPI) (Utilities|String|Append "[" (Utilities|String|ToString(Integer) _year) "-" (Utilities|String|ToString(Integer) _month) "-" (Utilities|String|ToString(Integer) _day) " " (Utilities|String|ToString(Integer) _hour) ":" (Utilities|String|ToString(Integer) _minute) ":" (Utilities|String|ToString(Integer) _second) "." (Utilities|String|ToString(Integer) _millisecond) "] [" Mod%20Name "]" Message) false))