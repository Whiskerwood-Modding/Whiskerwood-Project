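; Main-menu loader for the Short Night mod that registers its night-length setting through the mod API.
; On BeginPlay it adds English name and description strings, then registers the option after a short delay.
; It re-registers on language changes, using localized text with built-in fallbacks for empty entries.
; Disconnected leftover chains hold old debug display and SystemTunes writes, so this asset no longer changes night length itself.
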(event Custom|OnOptionChanged
  (params (optionId :type String) (Value :type String))
  (bind (_name _description) (CallFunction|GetLocalizedOption))
  (if (Utilities|Enum|Equal(Enum) optionId "settings.language")
    (Class|ModAPI|RegisterModOptions (Class|ModAPI|GetModAPI) (Variables|Default|GetNightLengthOptionId) _name (Variables|Default|GetOptionsValues) "5x" _description)))

(event EventBeginPlay
  (bind (_name _description) (CallFunction|GetLocalizedOption))
  (EventDispatchers|BindEventtoOnOptionChanged (Class|ModAPI|GetModAPI) (EventDispatchers|CreateEvent :!event Custom|OnOptionChanged))
  (CallFunction|AddNewStrings)
  (Utilities|FlowControl|Delay 0.2)
  (Class|ModAPI|RegisterModOptions (Class|ModAPI|GetModAPI) (Variables|Default|GetNightLengthOptionId) _name (Variables|Default|GetOptionsValues) "5x" _description))

(event EventTick
  (params (DeltaSeconds :type Float%20%28single-precision%29))
  ;[0.15 0.15 0.15 0.5] Temp/old stuff
)

(fn ConstructionScript)

(fn AddNewStrings
  (bind _nightlengthoptionid (Variables|Default|GetNightLengthOptionId))
  (Class|ModAPI|AddNewStrings (Class|ModAPI|GetModAPI) "en" (Utilities|Map|MakeMap (Utilities|String|StringToName (Utilities|String|Append "setting." _nightlengthoptionid ".name")) (Variables|Default|GetNightLengthName) (Utilities|String|StringToName (Utilities|String|Append "setting." _nightlengthoptionid ".description")) (Variables|Default|GetNightLengthDesc))))

(fn GetLocalizedOption
  (bind _returnvalue (Class|Backbone|GetLocManager))
  (bind _nightlengthname (Variables|Default|GetNightLengthName))
  (bind _nightlengthdesc (Variables|Default|GetNightLengthDesc))
  (bind _nightlengthoptionid (Variables|Default|GetNightLengthOptionId))
  (bind _returnvalue_2 (Utilities|String|Append "setting." _nightlengthoptionid ".description"))
  (bind _returnvalue_3 (Utilities|String|Append "setting." _nightlengthoptionid ".name"))
  (bind _returnvalue_4 (Utilities|String|StringToName _returnvalue_2))
  (bind _returnvalue_5 (Utilities|String|StringToName _returnvalue_3))
  (bind _returnvalue_6 (Class|LocManager|GetWordfromKey _returnvalue _returnvalue_4))
  (bind _returnvalue_7 (Class|LocManager|GetWordfromKey _returnvalue _returnvalue_5))
  (bind _returnvalue_8 (Utilities|Array|IsEmpty _returnvalue_6))
  (if (Utilities|Array|IsEmpty _returnvalue_7)
    (if _returnvalue_8
      (return _nightlengthname _nightlengthdesc)
      (else
        (return _nightlengthname _returnvalue_6)))
    (elif _returnvalue_8
      (return _returnvalue_7 _nightlengthdesc)
      (else
        (return _returnvalue_7 _returnvalue_6)))))