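; Main-menu loader for the HigherCropYields mod, which adds a crop yield option to the game's mod settings.
; On BeginPlay it adds English strings, registers the option after a short delay and writes the saved value's first character to GlobalCropYieldFactor in the SystemTunes DataTable.
; Option changes rewrite that factor, while language changes re-register the option with localized text, falling back to built-in defaults.
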(event Custom|OnOptionChanged
  (params (optionId :type String) (Value :type String))
  (bind (_name _description) (CallFunction|GetLocalizedOption))
  (if (Utilities|Enum|Equal(Enum) optionId "settings.language")
    (Class|ModAPI|RegisterModOptions (Class|ModAPI|GetModAPI) (Variables|Default|GetYieldOptionId) _name (Variables|Default|GetOptionsValues) (Variables|Default|GetDefaultOptionValue) _description)
    (elif (Utilities|Enum|Equal(Enum) optionId (Variables|Default|GetYieldOptionId))
      (Class|ModAPI|WriteDataTableValue (Class|ModAPI|GetModAPI) "SystemTunes" "GlobalCropYieldFactor" "floatValue" (Utilities|String|GetSubstring Value 0)))))

(event EventBeginPlay
  (bind (_name _description) (CallFunction|GetLocalizedOption))
  (EventDispatchers|BindEventtoOnOptionChanged (Class|ModAPI|GetModAPI) (EventDispatchers|CreateEvent :!event Custom|OnOptionChanged))
  (CallFunction|AddNewStrings)
  (Utilities|FlowControl|Delay 0.2)
  (Class|ModAPI|RegisterModOptions (Class|ModAPI|GetModAPI) (Variables|Default|GetYieldOptionId) _name (Variables|Default|GetOptionsValues) (Variables|Default|GetDefaultOptionValue) _description)
  (bind _returnvalue (Class|ModAPI|ReadModOptionValue (Class|ModAPI|GetModAPI) (Variables|Default|GetYieldOptionId) (Variables|Default|GetDefaultOptionValue)))
  (Class|ModAPI|WriteDataTableValue (Class|ModAPI|GetModAPI) "SystemTunes" "GlobalCropYieldFactor" "floatValue" (Utilities|String|GetSubstring _returnvalue 0)))

(fn ConstructionScript)

(fn AddNewStrings
  (bind _yieldoptionid (Variables|Default|GetYieldOptionId))
  (Class|ModAPI|AddNewStrings (Class|ModAPI|GetModAPI) "en" (Utilities|Map|MakeMap (Utilities|String|StringToName (Utilities|String|Append "setting." _yieldoptionid ".name")) (Variables|Default|GetYieldName) (Utilities|String|StringToName (Utilities|String|Append "setting." _yieldoptionid ".description")) (Variables|Default|GetYieldDesc))))

(fn GetLocalizedOption
  (bind _returnvalue (Class|Backbone|GetLocManager))
  (bind _yieldname (Variables|Default|GetYieldName))
  (bind _yielddesc (Variables|Default|GetYieldDesc))
  (bind _yieldoptionid (Variables|Default|GetYieldOptionId))
  (bind _returnvalue_2 (Utilities|String|Append "setting." _yieldoptionid ".description"))
  (bind _returnvalue_3 (Utilities|String|Append "setting." _yieldoptionid ".name"))
  (bind _returnvalue_4 (Utilities|String|StringToName _returnvalue_2))
  (bind _returnvalue_5 (Utilities|String|StringToName _returnvalue_3))
  (bind _returnvalue_6 (Class|LocManager|GetWordfromKey _returnvalue _returnvalue_4))
  (bind _returnvalue_7 (Class|LocManager|GetWordfromKey _returnvalue _returnvalue_5))
  (bind _returnvalue_8 (Utilities|Array|IsEmpty _returnvalue_6))
  (if (Utilities|Array|IsEmpty _returnvalue_7)
    (if _returnvalue_8
      (return _yieldname _yielddesc)
      (else
        (return _yieldname _returnvalue_6)))
    (elif _returnvalue_8
      (return _returnvalue_7 _yielddesc)
      (else
        (return _returnvalue_7 _returnvalue_6)))))