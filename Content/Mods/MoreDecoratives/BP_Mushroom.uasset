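; BP_Mushroom is a decorative mushroom from the MoreDecoratives mod whose fairy-light particles and point light follow the world's time of day.
; Every tick it looks up WorldTime_BP and acts only when the phase differs from the cached PreviousPhase.
; Mid day sets blue, short-lived Niagara particles and hides the light, while late night sets orange, longer-lived particles and shows it.
; Other phases leave the visuals unchanged.
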(event EventTick
  (params (DeltaSeconds :type Float%20%28single-precision%29))
  (bind _fx_fairylights (Variables|Default|GetFX_FairyLights))
  (bind _fx_fairylights_2 (Variables|Default|GetFX_FairyLights))
  (bind _fx_fairylights_3 (Variables|Default|GetFX_FairyLights))
  (bind _pointlight (Variables|Default|GetPointLight))
  (bind _returnvalue (Actor|GetActorOfClass "/Game/Code/Systems/WorldTime_BP.WorldTime_BP_C"))
  (Utilities|IsValid _returnvalue
    (:Is%20Valid
      (if (Utilities|Enum|NotEqual(Enum) (Variables|/Script/ProjectArco.WorldTime|Getm_currentPhase _returnvalue) (Variables|Default|GetPreviousPhase))
        (bind _output_get (Variables|Default|SetPreviousPhase (Variables|/Script/ProjectArco.WorldTime|Getm_currentPhase _returnvalue)))
        (switch Utilities|FlowControl|Switch|SwitchonEDayPhase _output_get
          (:MID_DAY
            (Components|Activation|SetActive _fx_fairylights true false)
            (Niagara|SetNiagaraVariable(LinearColor) _fx_fairylights_3 "FairyColor" (Math|Color|MakeColor 0.07551 0.053928 0.848695 0.5))
            (Niagara|SetNiagaraVariable(Float) _fx_fairylights_2 "Lifetime" 5.0)
            (Rendering|SetVisibility _pointlight false true))
          (:LATE_NIGHT
            (Components|Activation|SetActive _fx_fairylights true false)
            (Niagara|SetNiagaraVariable(LinearColor) _fx_fairylights_3 "FairyColor" (Math|Color|MakeColor 1.0 0.46832 0.0))
            (Niagara|SetNiagaraVariable(Float) _fx_fairylights_2 "Lifetime" 3e+01)
            (Rendering|SetVisibility _pointlight true true)))))))

(fn ConstructionScript)