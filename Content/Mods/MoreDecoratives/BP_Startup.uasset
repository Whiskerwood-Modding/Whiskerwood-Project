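; Startup Blueprint for the MoreDecoratives mod that registers new slot decoratives such as walls, lights, logs and a doorway on BeginPlay.
; CreateNewSlotDecorative uses the mod API to write slot-decorative and icon DataTable rows, serializing asset references as path strings, and collects display names.
; Those names then go into the English localization table in one call, with failures logged.
; Cobblestones, fountain and invisible wall registrations are left disconnected, and WriteStringsRow is unused.
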(event EventBeginPlay
  (Utilities|FlowControl|Sequence
    (:then_0
      (CallFunction|CreateNewSlotDecorative "decorslot_bookshelf" (Utilities|Struct|MakeSlotDecorative "moredecoratives.slotdecorative.bookshelf" "/Game/Mods/MoreDecoratives/BP_Bookshelf.BP_Bookshelf_C" "INNER_EDGE" "OPEN") "/Game/Assets/Rendered/Icons/Building/decorslot_lamp.decorslot_lamp" "Bookshelf")
      (CallFunction|CreateNewSlotDecorative "decorslot_mushroom" (Utilities|Struct|MakeSlotDecorative "moredecoratives.slotdecorative.mushroom" "/Game/Mods/MoreDecoratives/BP_Mushroom.BP_Mushroom_C" "INNER_EDGE" "OPEN") "/Game/Assets/Rendered/Icons/Building/decorslot_lamp.decorslot_lamp" "Mushroom")
      (CallFunction|CreateNewSlotDecorative "decorslot_leafywall" (Utilities|Struct|MakeSlotDecorative "moredecoratives.slotdecorative.leafywall" "/Game/Mods/MoreDecoratives/BP_HedgeFence.BP_HedgeFence_C") "/Game/Assets/Rendered/Icons/Building/decorslot_lamp.decorslot_lamp" "Leafy Wall")
      (CallFunction|CreateNewSlotDecorative "decorslot_log" (Utilities|Struct|MakeSlotDecorative "moredecoratives.slotdecorative.log" "/Game/Mods/MoreDecoratives/BP_Log.BP_Log_C") "/Game/Assets/Rendered/Icons/Building/decorslot_lamp.decorslot_lamp" "Log")
      (CallFunction|CreateNewSlotDecorative "decorslot_lumber" (Utilities|Struct|MakeSlotDecorative "moredecoratives.slotdecorative.lumber" "/Game/Mods/MoreDecoratives/BP_Lumber.BP_Lumber_C" "INNER_EDGE" "OPEN") "/Game/Assets/Rendered/Icons/Building/decorslot_lamp.decorslot_lamp" "Lumber")
      (CallFunction|CreateNewSlotDecorative "decorslot_tallwall" (Utilities|Struct|MakeSlotDecorative "moredecoratives.slotdecorative.tallwall" "/Game/Mods/MoreDecoratives/BP_TallCobblestoneWall.BP_TallCobblestoneWall_C") "/Game/Assets/Rendered/Icons/Building/decorslot_lamp.decorslot_lamp" "Tall Wall")
      (CallFunction|CreateNewSlotDecorative "decorslot_lamppost" (Utilities|Struct|MakeSlotDecorative "moredecoratives.slotdecorative.lamppost" "/Game/Mods/MoreDecoratives/BP_Lamppost.BP_Lamppost_C" "INNER_EDGE" "OPEN") "/Game/Assets/Rendered/Icons/Building/decorslot_lamp.decorslot_lamp" "Lamppost")
      (CallFunction|CreateNewSlotDecorative "decorslot_fairylights" (Utilities|Struct|MakeSlotDecorative "moredecoratives.slotdecorative.fairylights" "/Game/Mods/MoreDecoratives/BP_FairyLights.BP_FairyLights_C" "INNER_EDGE" "OPEN") "/Game/Assets/Rendered/Icons/Building/decorslot_lamp.decorslot_lamp" "Fairy Lights")
      (CallFunction|CreateNewSlotDecorative "decorslot_lantern" (Utilities|Struct|MakeSlotDecorative "moredecoratives.slotdecorative.lantern" "/Game/Mods/MoreDecoratives/BP_Lantern.BP_Lantern_C" "INNER_EDGE" "OPEN") "/Game/Assets/Rendered/Icons/Building/decorslot_lamp.decorslot_lamp" "Lantern")
      (CallFunction|CreateNewSlotDecorative "decorslot_bidirectionaldoorway" (Utilities|Struct|MakeSlotDecorative "moredecoratives.slotdecorative.bidirectionalDoorway" "/Game/Mods/MoreDecoratives/BP_BidirectionalDoorway.BP_BidirectionalDoorway_C" "OUTER_EDGE" "OPEN") "/Game/Assets/Rendered/Icons/Building/decorslot_onewaygate.decorslot_onewaygate" "Doorway")
      (CallFunction|CreateNewSlotDecorative "decorslot_brickwall" (Utilities|Struct|MakeSlotDecorative "moredecoratives.slotdecorative.brickwall" "/Game/Mods/MoreDecoratives/BP_BrickWall.BP_BrickWall_C") "/Game/Assets/Rendered/Icons/Building/decorslot_lamp.decorslot_lamp" "Brick Wall"))
    (:then_1
      (bind _returnvalue (Class|ModAPI|AddNewStrings (Class|ModAPI|GetModAPI) "en" (Variables|Default|GetLoc%20Strings)))
      (if (not _returnvalue)
        (CallFunction|LogMessage "failed to add to en table")))))

(fn ConstructionScript)

(fn LogMessage
  (params (Message :type String))
  (bind _returnvalue (Math|DateTime|Now))
  (bind (_year _month _day _hour _minute _second _millisecond) (Math|DateTime|BreakDateTime _returnvalue))
  (if (Variables|Default|GetEnable%20Logging?)
    (Class|ModAPI|LogMessage (Class|ModAPI|GetModAPI) (Utilities|String|Append "[" (Utilities|String|ToString(Integer) _year) "-" (Utilities|String|ToString(Integer) _month) "-" (Utilities|String|ToString(Integer) _day) " " (Utilities|String|ToString(Integer) _hour) ":" (Utilities|String|ToString(Integer) _minute) ":" (Utilities|String|ToString(Integer) _second) "." (Utilities|String|ToString(Integer) _millisecond) "] [" (Variables|Default|GetMod%20Name) "] " Message) false)))

(fn ConstructBPRef
  (params (ClassRef :type Actor%20Class%20Reference))
  (return (Utilities|String|Append "/Script/Engine.BlueprintGeneratedClass'" (.pathstring (Class|KismetSystemLibrary|GetSoftClassPath ClassRef)) "'")))

(fn WriteStringsRow
  (params (Value :type String) (Row%20Id :type Name))
  (bind _returnvalue (Class|ModAPI|GetModAPI))
  (bind _stringsdt (LocalVariables|GetStringsDT))
  (bind _returnvalue_2 (Class|ModAPI|AddDataTableRow _returnvalue _stringsdt Row%20Id))
  (if _returnvalue_2
    (bind _returnvalue_3 (Class|ModAPI|WriteDataTableValue _returnvalue _stringsdt Row%20Id "Value" Value))
    (if (not _returnvalue_3)
      (CallFunction|LogMessage "failed to write strings DT \"Value\""))
    (else
      (CallFunction|LogMessage "failed to add strings DT row"))))

(fn WriteIconsRow
  (params (Icon :type Icon%20Data%20Row%20Base%20Structure) (Row%20Id :type Name))
  (bind _returnvalue (Class|ModAPI|GetModAPI))
  (bind _icons_buildings (LocalVariables|GetIcons_Buildings))
  (Class|ModAPI|AddDataTable _returnvalue _icons_buildings "/Game/Data/Icons/Icons_Buildings.Icons_Buildings")
  (bind _returnvalue_2 (Class|ModAPI|AddDataTableRow _returnvalue _icons_buildings Row%20Id))
  (if _returnvalue_2
    (bind _returnvalue_3 (Class|ModAPI|WriteDataTableValue _returnvalue _icons_buildings Row%20Id "Icon" (CallFunction|ConstructIconRef (.icon Icon))))
    (if (not _returnvalue_3)
      (CallFunction|LogMessage "failed to add icon to Icons_Buildings row"))
    (else
      (CallFunction|LogMessage "failed to add row to Icons_Buildings DT"))))

(fn ConstructIconRef
  (params (Icon :type Texture%202D%20Object%20Reference))
  (return (Utilities|String|Append "/Script/Engine.Texture2D'" (.pathstring (Utilities|GetSoftObjectPath Icon)) "'")))

(fn WriteSlotDecorativesRow
  (params (RowId :type Name) (SlotDecorative :type Slot%20Decorative%20Structure))
  (bind _returnvalue (Class|ModAPI|GetModAPI))
  (bind _returnvalue_2 (Class|ModAPI|AddDataTableRow _returnvalue (LocalVariables|GetSlotDecoratives) RowId))
  (if _returnvalue_2
    (bind _returnvalue_3 (Class|ModAPI|WriteDataTableValue _returnvalue (LocalVariables|GetSlotDecoratives) RowId "LocKey" (.lockey SlotDecorative)))
    (if _returnvalue_3
      (bind _returnvalue_4 (Class|ModAPI|WriteDataTableValue _returnvalue (LocalVariables|GetSlotDecoratives) RowId "decorativeActor" (CallFunction|ConstructBPRef (.decorativeactor SlotDecorative))))
      (if _returnvalue_4
        (bind _returnvalue_5 (Class|ModAPI|WriteDataTableValue _returnvalue (LocalVariables|GetSlotDecoratives) RowId "desiredSubSlot" (Utilities|String|EnumtoString (.desiredsubslot SlotDecorative))))
        (if _returnvalue_5
          (bind _returnvalue_6 (Class|ModAPI|WriteDataTableValue _returnvalue (LocalVariables|GetSlotDecoratives) RowId "pathingEffect" (Utilities|String|EnumtoString (.pathingeffect SlotDecorative))))
          (if (not _returnvalue_6)
            (CallFunction|LogMessage "failed to write to slot decorative"))
          (else
            (CallFunction|LogMessage "failed to write to slot decorative")))
        (else
          (CallFunction|LogMessage "failed to write to slot decorative")))
      (else
        (CallFunction|LogMessage "failed to write to slot decorative")))
    (else
      (CallFunction|LogMessage "failed to add slot deco DT row"))))

(fn CreateNewSlotDecorative
  (params (RowId :type Name) (Details :type Slot%20Decorative%20Structure) (Icon :type Texture%202D%20Object%20Reference) (Name :type String))
  (CallFunction|WriteSlotDecorativesRow RowId (Utilities|Struct|MakeSlotDecorative (.lockey Details) (.decorativeactor Details) (.desiredsubslot Details) (.pathingeffect Details) 0))
  (CallFunction|WriteIconsRow (Utilities|Struct|MakeIconDataRowBase Icon) RowId)
  (Utilities|Map|Add (Variables|Default|GetLoc%20Strings) (Utilities|String|StringToName (.lockey Details)) Name))