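; Startup Blueprint for the zhLocalization mod that registers localized strings for the "dev" and "zh" languages on BeginPlay.
; AddNewStrings reads a mod text file through the mod API, skips the header, splits entries at commas into an ID-to-text map and submits it.
; The NewStrings map is never cleared, so the zh submission also carries dev entries unless overwritten.
; A LogMessages flag gates mod-prefixed logging throughout.
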(event EventBeginPlay
  (CallFunction|AddNewStrings "dev.txt" "dev")
  (CallFunction|AddNewStrings "zh.txt" "zh")
  (CallFunction|Log "Localized strings!"))

(fn ConstructionScript)

(fn Log
  (params (Message :type String))
  (if (Variables|Default|GetLog%20Messages?)
    (Class|ModAPI|LogMessage (Class|ModAPI|GetModAPI) (Utilities|String|Append "[" (Variables|Default|GetMod%20Name) "] " Message) true)))

(fn AddNewStrings
  (params (filename :type String) (language%20id :type Name))
  (bind _returnvalue (Class|ModAPI|ReadModTextFile (Class|ModAPI|GetModAPI) (Variables|Default|GetMod%20Name) filename))
  (CallFunction|Log _returnvalue)
  (for (_array_element _array_index) (Utilities|String|ParseIntoArray _returnvalue " 
")
    (CallFunction|Log _array_element)
    ;[0.15 0.15 0.15 0.5] Don't parse header
    (if (not (== _array_index 0))
      (if (.ReturnValue (Utilities|String|Split _array_element ","))
        (Utilities|Map|Add (LocalVariables|GetNewStrings) (Utilities|String|StringToName (.LeftS (Utilities|String|Split _array_element ","))) (.RightS (Utilities|String|Split _array_element ",")))
        (else
          (CallFunction|Log "failed to split")))))
  (bind _returnvalue_2 (Class|ModAPI|AddNewStrings (Class|ModAPI|GetModAPI) language%20id (LocalVariables|GetNewStrings)))
  (if _returnvalue_2
    (CallFunction|Log "added new strings")
    (else
      (CallFunction|Log "failed to add new zh strings"))))