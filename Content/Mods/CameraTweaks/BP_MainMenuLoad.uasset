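; Main menu loader for the CameraTweaks mod that registers its configurable options with the mod API.
; On BeginPlay it adds each option's default name and description as English strings under setting.<id> keys, then registers the options after a short delay.
; Registration prefers text from the localization manager, falling back to each option's own text when empty.
; A language setting change re-registers all options to refresh the displayed text.
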(event Custom|OnOptionChanged
  (params (optionId :type String) (Value :type String))
  (if (Utilities|Enum|Equal(Enum) optionId "settings.language")
    (CallFunction|RegisterModOptions)))

(event EventBeginPlay
  (EventDispatchers|BindEventtoOnOptionChanged (Class|ModAPI|GetModAPI) (EventDispatchers|CreateEvent :!event Custom|OnOptionChanged))
  (for _array_element (Variables|Default|GetOptions)
    (CallFunction|MakeLocalizedMap _array_element))
  (Class|ModAPI|AddNewStrings (Class|ModAPI|GetModAPI) "en" (Variables|Default|GetLocalized%20Map))
  (Utilities|FlowControl|Delay 0.2)
  (CallFunction|RegisterModOptions))

(fn ConstructionScript)

(fn RegisterModOptions
  (bind _returnvalue (Class|ModAPI|GetModAPI))
  (bind _returnvalue_2 (Class|ModAPI|GetModAPI))
  (for _array_element (Variables|Default|GetOptions)
    (bind _output_get (LocalVariables|SetCurrentOption _array_element))
    (bind (_name _description) (CallFunction|GetLocalizedOption (.optionid _output_get)))
    (bind _output_get_2 (LocalVariables|SetLocalizedName _name))
    (bind _output_get_3 (LocalVariables|SetLocalizedDesc _description))
    (if (Utilities|Array|IsEmpty _output_get_2)
      (if (Utilities|Array|IsEmpty _output_get_3)
        (Class|ModAPI|RegisterModOptions _returnvalue (.optionid (LocalVariables|GetCurrentOption)) (.optiondisplayname (LocalVariables|GetCurrentOption)) (.optionvalues (LocalVariables|GetCurrentOption)) (.optiondefaultvalue (LocalVariables|GetCurrentOption)) (.optiondescription (LocalVariables|GetCurrentOption)))
        (else
          (Class|ModAPI|RegisterModOptions _returnvalue (.optionid (LocalVariables|GetCurrentOption)) (.optiondisplayname (LocalVariables|GetCurrentOption)) (.optionvalues (LocalVariables|GetCurrentOption)) (.optiondefaultvalue (LocalVariables|GetCurrentOption)) (LocalVariables|GetLocalizedDesc))))
      (elif (Utilities|Array|IsEmpty _output_get_3)
        (Class|ModAPI|RegisterModOptions _returnvalue_2 (.optionid (LocalVariables|GetCurrentOption)) (LocalVariables|GetLocalizedName) (.optionvalues (LocalVariables|GetCurrentOption)) (.optiondefaultvalue (LocalVariables|GetCurrentOption)) (.optiondescription (LocalVariables|GetCurrentOption)))
        (else
          (Class|ModAPI|RegisterModOptions _returnvalue_2 (.optionid (LocalVariables|GetCurrentOption)) (LocalVariables|GetLocalizedName) (.optionvalues (LocalVariables|GetCurrentOption)) (.optiondefaultvalue (LocalVariables|GetCurrentOption)) (LocalVariables|GetLocalizedDesc)))))))

(fn GetLocalizedOption
  (params (Option%20Id :type String))
  (bind _returnvalue (Class|Backbone|GetLocManager))
  (return (Class|LocManager|GetWordfromKey _returnvalue (Utilities|String|StringToName (Utilities|String|Append "setting." Option%20Id ".name"))) (Class|LocManager|GetWordfromKey _returnvalue (Utilities|String|StringToName (Utilities|String|Append "setting." Option%20Id ".description")))))

(fn MakeLocalizedMap
  (params (Option :type ST%20Camera%20Tweaks%20Options%20Structure))
  (bind (_optionid _optiondisplayname _optiondefaultvalue _optionvalues _optiondescription) (Utilities|Struct|BreakST_CameraTweaksOptions Option))
  (Utilities|Map|Add (Variables|Default|GetLocalized%20Map) (Utilities|String|StringToName (Utilities|String|Append "setting." _optionid ".name")) _optiondisplayname)
  (Utilities|Map|Add (Variables|Default|GetLocalized%20Map) (Utilities|String|StringToName (Utilities|String|Append "setting." _optionid ".description")) _optiondescription))